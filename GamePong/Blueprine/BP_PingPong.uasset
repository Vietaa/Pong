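; VR player Blueprint for a ping-pong game, handling hand poses, turning and UI clicking.
; Grip inputs set left and right fist flags, and the right trigger drives the WidgetInteraction as a left mouse click.
; The right thumbstick axis yaws the Vr component by SnapRotation, throttled by a DoOnce with delayed reset.
; BeginPlay sets floor tracking origin; racket spawn-and-attach logic is present but never runs.
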(event `InputAction|GrapRightFist`
  (params (Key :type "Key Structure"))
  ;[1 1 1] AnimtionPickUp
  (:`Pressed`
    (set `self.RightMakeFist` true))
  (:`Released`
    (set `self.RightMakeFist` false)))

(event `InputAction|GrapLightFist`
  (params (Key :type "Key Structure"))
  ;[1 1 1] AnimtionPickUp
  (:`Pressed`
    (set `self.LightMakeFist` true))
  (:`Released`
    (set `self.LightMakeFist` false)))

(event `InputAxis|MotionRotationThumRigthY`
  (params (AxisValue :type "Float (single-precision)"))
  (bind (_returnvalue_roll _returnvalue_pitch _returnvalue_yaw) (`KismetMathLibrary.BreakRotator` (`SceneComponent.K2_GetComponentRotation` (`self.Vr`))))
  ;[1 1 1] SnapRotation
  (`/Engine/EditorBlueprintResources/StandardMacros.DoOnce` false :!label _label
    (:`Completed`
      (`|ExecutionSequence`
        (:`then_0`
          (`SceneComponent.K2_SetWorldRotation` (`self.Vr`) (`KismetMathLibrary.MakeRotator` 0.0 0.0 (+ _returnvalue_yaw (* (`self.SnapRotation`) AxisValue))) false false))
        (:`then_1`
          (`KismetSystemLibrary.Delay` 0.2)
          (goto _label :!via `Reset`))))))

(event `InputAction|TriggerRight`
  (params (Key :type "Key Structure"))
  (bind _widgetinteraction (`self.WidgetInteraction`))
  ;[1 1 1] ConvertTrigger
  (:`Pressed`
    (set `WidgetInteractionComponent.bShowDebug` false _widgetinteraction)
    (`WidgetInteractionComponent.PressPointerKey` _widgetinteraction "LeftMouseButton"))
  (:`Released`
    (set `WidgetInteractionComponent.bShowDebug` false _widgetinteraction)
    (`WidgetInteractionComponent.ReleasePointerKey` _widgetinteraction "LeftMouseButton")))

(event `CustomEvent_1`
  ;[1 1 1] SnapRotation
  (`KismetSystemLibrary.PrintString` "Hello"))

(event `CustomEvent_0`
  ;[1 1 1] SnapRotation
  (`self.CustomEvent_1`))

(event `self.ReceiveBeginPlay`
  ;[1 0.02604 0.02604] LocationCamera and Spawn Racket
  (`HeadMountedDisplayFunctionLibrary.SetTrackingOrigin` "Floor"))

(fn `UserConstructionScript`)