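; Menu controller for the Pong game that shows the play menu and relays host and join requests.
; On BeginPlay it caches SV_GameInstance and, only on the server, creates the UI_WigetPlay widget, hands it a self-reference and sets a UI-only cursor input mode.
; ClientHostSession and ClientJoinSession forward to the game instance's HostSever and JoinSession functions.
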(event `self.ReceiveBeginPlay`
  (bind _returnvalue (`GameplayStatics.GetPlayerController` 0))
  ;[1 1 1] Create UI
  (bind _assv_game_instance (cast `/Game/Pong/GamePong/Framework/SV_GameInstance` (`GameplayStatics.GetGameInstance`)))
  (set `self.GameInstance` _assv_game_instance)
  (if (`KismetSystemLibrary.IsServer`)
    (`/Engine/EditorBlueprintResources/StandardMacros.IsValid` (`self.Widget`)
      (:`Is Valid`
        _)
      (:`Is Not Valid`
        (bind _returnvalue_2 (`|CreateWidget` "/Game/Pong/GamePong/UI/UI_WigetPlay.UI_WigetPlay_C" (`GameplayStatics.GetPlayerController` 0)))
        (`UserWidget.AddToViewport` _returnvalue_2 0)))
    (bind _output_get (set `self.Widget` _returnvalue_2))
    (set `/Game/Pong/GamePong/UI/UI_WigetPlay.MenuController` self (`self.Widget`))
    (set `PlayerController.bShowMouseCursor` true _returnvalue)
    (`WidgetBlueprintLibrary.SetInputMode_UIOnlyEx` _returnvalue _output_get)))

(event `ClientHostSession`
  ;[1 1 1] ConnectSever
  (`/Game/Pong/GamePong/Framework/SV_GameInstance.Host Sever` (`self.GameInstance`)))

(event `ClientJoinSession`
  ;[1 1 1] ConnectSever
  (`/Game/Pong/GamePong/Framework/SV_GameInstance.Join Session` (`self.GameInstance`)))

(fn `UserConstructionScript`)