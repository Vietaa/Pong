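; Main game actor for networked Pong that spawns the ball and handles scoring.
; On authority BeginPlay, it spawns a physics ball and caches two raised spawn transforms; a new-game event picks the one nearer the ball.
; Goal hit components destroy the ball, respawn it after a short delay and update GS_GameState score and rounds.
; ROS/MTC-suffixed events relay results to two UI_Goald widgets, while actor hits spawn impact particles.
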(event `SetTransFrom`
  ;[1 1 1] Set Transfrom Spawn ball
  (set `self.TransfromSpawnball1` (`KismetMathLibrary.MakeTransform` (`KismetMathLibrary.MakeVector` (.x (.location (`SceneComponent.K2_GetComponentToWorld` (`self.BallTargetPoint`)))) (.y (.location (`SceneComponent.K2_GetComponentToWorld` (`self.BallTargetPoint`)))) (+ (.z (.location (`SceneComponent.K2_GetComponentToWorld` (`self.BallTargetPoint`)))) 50.0)) (.rotation (`SceneComponent.K2_GetComponentToWorld` (`self.BallTargetPoint`))) (.scale (`SceneComponent.K2_GetComponentToWorld` (`self.BallTargetPoint`)))))
  (set `self.TransfromSpawnBall2` (`KismetMathLibrary.MakeTransform` (`KismetMathLibrary.MakeVector` (.x (.location (`SceneComponent.K2_GetComponentToWorld` (`self.BallSpawn2`)))) (.y (.location (`SceneComponent.K2_GetComponentToWorld` (`self.BallSpawn2`)))) (+ (.z (.location (`SceneComponent.K2_GetComponentToWorld` (`self.BallSpawn2`)))) 90.0)) (.rotation (`SceneComponent.K2_GetComponentToWorld` (`self.BallSpawn2`))) (.scale (`SceneComponent.K2_GetComponentToWorld` (`self.BallSpawn2`))))))

(event `SpawnNewGameROS`
  (bind _returnvalue (`self.K2_GetActorLocation` (`self.BP_Ball`)))
  (bind _location (.location (`self.TransfromSpawnball1`)))
  (bind _location_2 (.location (`self.TransfromSpawnBall2`)))
  ;[1 1 1] SpawnnewGame
  (if (> (`KismetMathLibrary.Abs` (`KismetMathLibrary.VSize` (- _returnvalue _location_2))) (`KismetMathLibrary.Abs` (`KismetMathLibrary.VSize` (- _returnvalue _location))))
    (`self.Spawn New Ball Event ROS` (`KismetMathLibrary.MakeTransform` _location (.rotation (`self.TransfromSpawnball1`)) (.scale (`self.TransfromSpawnball1`))))
    (else
      (`self.Spawn New Ball Event ROS` (`KismetMathLibrary.MakeTransform` _location_2 (.rotation (`self.TransfromSpawnBall2`)) (.scale (`self.TransfromSpawnBall2`)))))))

(event `SpawnBallBecauseScore ROS`
  (params (TransfromSpawn :type "Transform Structure"))
  ;[1 1 1] SpawnBallBecauseScore
  (`self.Spawn New Ball Event ROS` TransfromSpawn))

(event `self.ReceiveBeginPlay`
  ;[1 1 1] Beginplay
  (`/Engine/EditorBlueprintResources/ActorMacros.Switch Has Authority`
    (:`Authority`
      (`self.Spawn New Ball Event ROS` (`SceneComponent.K2_GetComponentToWorld` (`self.BallTargetPoint`)))
      (`self.SetTransFrom`))))

(event `Spawn New Ball Event ROS`
  (params (TransfromSpawn :type "Transform Structure"))
  ;[1 1 1] SpawnNewBall
  (`ActorComponent.Activate` (`self.Spawner_ParticleSystem`) true)
  (bind _returnvalue (`|SpawnActorFromClass` "/Game/Pong/GamePong/Blueprine/BP_BallProjectile.BP_BallProjectile_C" TransfromSpawn "AlwaysSpawn" "OverrideRootScale" null 300.0 2500.0 150.0 5.0 0.15 null))
  (bind _output_get (set `self.BP_Ball` _returnvalue))
  (set `/Game/Pong/GamePong/Blueprine/BP_BallProjectile.BP_Main` self _output_get)
  (`ActorComponent.Deactivate` (`self.Spawner_ParticleSystem`))
  (`/Game/Pong/GamePong/Blueprine/BP_BallProjectile.Enable Physics Simulation ROS` _returnvalue))

(event `self.Hit1.OnComponentHit`
  (params (HitComponent :type "PrimitiveComponent Object Reference") (OtherActor :type "Actor Object Reference") (OtherComp :type "PrimitiveComponent Object Reference") (NormalImpulse :type "Vector Structure") (Hit :type "HitResult Structure (by ref)"))
  ;[1 1 1] Hit Check Score
  (bind _asbp_ball_projectile (cast `/Game/Pong/GamePong/Blueprine/BP_BallProjectile` OtherActor))
  (`self.K2_DestroyActor` _asbp_ball_projectile)
  (bind _output_get (set `self.TransfromSpawnBall FollowScore` (`self.TransfromSpawnBall2`)))
  (`KismetSystemLibrary.Delay` 0.2)
  (`self.SpawnBallBecauseScore ROS` _output_get)
  (`self.CheckRoundAndScorePlayer1 ROS`))

(event `self.Hit2.OnComponentHit`
  (params (HitComponent :type "PrimitiveComponent Object Reference") (OtherActor :type "Actor Object Reference") (OtherComp :type "PrimitiveComponent Object Reference") (NormalImpulse :type "Vector Structure") (Hit :type "HitResult Structure (by ref)"))
  ;[1 1 1] Hit Check Score
  (bind _asbp_ball_projectile (cast `/Game/Pong/GamePong/Blueprine/BP_BallProjectile` OtherActor))
  (`self.K2_DestroyActor` _asbp_ball_projectile)
  (bind _output_get (set `self.TransfromSpawnBall FollowScore` (`self.TransfromSpawnball1`)))
  (`KismetSystemLibrary.Delay` 0.2)
  (`self.SpawnBallBecauseScore ROS` _output_get)
  (`self.CheckRoundAndscorePlayer2 ROS`))

(event `self.ReceiveHit`
  (params (MyComp :type "PrimitiveComponent Object Reference") (Other :type "Actor Object Reference") (OtherComp :type "PrimitiveComponent Object Reference") (bSelfMoved :type Boolean) (HitLocation :type "Vector Structure") (HitNormal :type "Vector Structure") (NormalImpulse :type "Vector Structure") (Hit :type "HitResult Structure (by ref)"))
  (bind (_bblockinghit _binitialoverlap _time _distance _location _impactpoint _normal) (`GameplayStatics.BreakHitResult` Hit))
  ;[1 1 1] Hit
  (cast `/Game/Pong/GamePong/Blueprine/BP_BallProjectile` Other)
  (`/Engine/EditorBlueprintResources/StandardMacros.DoOnce` false :!label _label
    (:`Completed`
      (`GameplayStatics.SpawnEmitterAtLocation` "/Game/Assets/Particles/PS_BallCollisionImpact.PS_BallCollisionImpact" (+ _location (* _normal 5.0)) (`KismetMathLibrary.MakeRotFromX` _normal))
      (`self.Reset Hit Detection`))))

(event `Reset Hit Detection`
  ;[1 1 1] Hit
  (goto _label :!via `Reset`))

(event `CheckRoundAndScorePlayer1 ROS`
  ;[1 1 1] CheckRoundandScore(ShowScore)
  (bind _asgs_game_state (cast `/Game/Pong/GamePong/Framework/GS_GameState` (`GameplayStatics.GetGameState`)))
  (`/Game/Pong/GamePong/Framework/GS_GameState.GS_CheckSocrePlayer1ROS` _asgs_game_state)
  (`/Game/Pong/GamePong/Framework/GS_GameState.GS_CheckRound1ROS` _asgs_game_state)
  (bind (_scoreplayer1 _scoreplayer2 _roundplayer1 _roundplayer2) (`/Game/Pong/GamePong/Framework/GS_GameState.Show Check` _asgs_game_state))
  (`self.UpdateScoreInUI MTC` _scoreplayer1 _scoreplayer2 _roundplayer1 _roundplayer2))

(event `CheckRoundAndscorePlayer2 ROS`
  ;[1 1 1] CheckRoundandScore(ShowScore)
  (bind _asgs_game_state (cast `/Game/Pong/GamePong/Framework/GS_GameState` (`GameplayStatics.GetGameState`)))
  (`/Game/Pong/GamePong/Framework/GS_GameState.GS_CheckScorePlayer2ROS` _asgs_game_state)
  (`/Game/Pong/GamePong/Framework/GS_GameState.GS_CheckRound2ROS` _asgs_game_state)
  (bind (_scoreplayer1 _scoreplayer2 _roundplayer1 _roundplayer2) (`/Game/Pong/GamePong/Framework/GS_GameState.Show Check` _asgs_game_state))
  (`self.UpdateScoreInUI MTC` _scoreplayer1 _scoreplayer2 _roundplayer1 _roundplayer2))

(event `UpdateScoreInUI MTC`
  (params (ScorePlayer1 :type Integer) (ScorePlayer2 :type Integer) (RoundPlayer1 :type Integer) (RoundPlayer2 :type Integer))
  ;[1 1 1] UpdateScoreInUI
  (`|ExecutionSequence`
    (:`then_0`
      (bind _asui_goald (cast `/Game/Pong/GamePong/Blueprine/UI_Goald` (`WidgetComponent.GetUserWidgetObject` (`self.Widget1`))))
      (`/Game/Pong/GamePong/Blueprine/UI_Goald.UI_UpDateGoaldAndRound MTC` _asui_goald ScorePlayer1 ScorePlayer2 RoundPlayer1 RoundPlayer2))
    (:`then_1`
      (bind _asui_goald_2 (cast `/Game/Pong/GamePong/Blueprine/UI_Goald` (`WidgetComponent.GetUserWidgetObject` (`self.Widget2`))))
      (`/Game/Pong/GamePong/Blueprine/UI_Goald.UI_UpDateGoaldAndRound MTC` _asui_goald_2 ScorePlayer1 ScorePlayer2 RoundPlayer1 RoundPlayer2))))

(fn `UserConstructionScript`)