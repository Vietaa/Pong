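; VR player character for the pong game, giving the player two rackets and a ball.
; BeginPlay sets floor tracking, attaches BP_Racket actors in place of both hidden hands, and spawns a BP_BallProjectile, which SpawnActor can also trigger.
; The ball and right racket receive a reference back to the character.
; Input drives fist-grip flags, thumbstick snap rotation throttled by DoOnce and Delay, and right-trigger widget clicks.
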(event `InputAction|GrapRightFist`
  (params (Key :type "Key Structure"))
  ;[1 1 1] AnimtionPickUp
  (:`Pressed`
    (set `self.RightMakeFist` true))
  (:`Released`
    (set `self.RightMakeFist` false)))

(event `InputAction|GrapLightFist`
  (params (Key :type "Key Structure"))
  ;[1 1 1] AnimtionPickUp
  (:`Pressed`
    (set `self.LightMakeFist` true))
  (:`Released`
    (set `self.LightMakeFist` false)))

(event `InputAxis|MotionRotationThumRigthY`
  (params (AxisValue :type "Float (single-precision)"))
  (bind (_returnvalue_roll _returnvalue_pitch _returnvalue_yaw) (`KismetMathLibrary.BreakRotator` (`SceneComponent.K2_GetComponentRotation` (`self.Vr`))))
  ;[1 1 1] SnapRotation
  (`/Engine/EditorBlueprintResources/StandardMacros.DoOnce` false :!label _label
    (:`Completed`
      (`|ExecutionSequence`
        (:`then_0`
          (`SceneComponent.K2_SetWorldRotation` (`self.Vr`) (`KismetMathLibrary.MakeRotator` 0.0 0.0 (+ _returnvalue_yaw (* (`self.SnapRotation`) AxisValue))) false false))
        (:`then_1`
          (`KismetSystemLibrary.Delay` 0.2)
          (goto _label :!via `Reset`))))))

(event `InputAction|TriggerRight`
  (params (Key :type "Key Structure"))
  (bind _widgetinteraction (`self.WidgetInteraction`))
  ;[1 1 1] ConvertTrigger
  (:`Pressed`
    (set `WidgetInteractionComponent.bShowDebug` false _widgetinteraction)
    (`WidgetInteractionComponent.PressPointerKey` _widgetinteraction "LeftMouseButton"))
  (:`Released`
    (set `WidgetInteractionComponent.bShowDebug` false _widgetinteraction)
    (`WidgetInteractionComponent.ReleasePointerKey` _widgetinteraction "LeftMouseButton")))

(event `SpawnActor`
  (bind _returnvalue (`self.GetTransform`))
  ;[1 0.02604 0.02604] LocationCamera and Spawn Racket
  (bind _returnvalue_2 (`|SpawnActorFromClass` "/Game/Pong/GamePong/Blueprine/BP_BallProjectile.BP_BallProjectile_C" (`KismetMathLibrary.MakeTransform` (`KismetMathLibrary.MakeVector` (.x (.location _returnvalue)) (+ (.y (.location _returnvalue)) 20.0) (.z (.location _returnvalue))) (.rotation _returnvalue) (0.2 0.2 0.2)) "Undefined" "OverrideRootScale" null 300.0 2500.0 200.0 2.0 0.15 null :!label _label_2))
  (bind _output_get (set `self.Bp_Ball` _returnvalue_2))
  (set `/Game/Pong/GamePong/Blueprine/BP_BallProjectile.BP_Character` self _output_get))

(event `self.ReceiveBeginPlay`
  (bind _right (`self.Right`))
  (bind _left (`self.Left`))
  (bind _returnvalue (`SceneComponent.K2_GetComponentLocation` (`self.TeleportArrowRotation`)))
  ;[1 0.02604 0.02604] LocationCamera and Spawn Racket
  (`HeadMountedDisplayFunctionLibrary.SetTrackingOrigin` "Floor")
  (`|ExecutionSequence`
    (:`then_0`
      (bind _returnvalue_2 (`|SpawnActorFromClass` "/Game/Pong/GamePong/Blueprine/BP_Racket.BP_Racket_C" (`KismetMathLibrary.MakeTransform` _returnvalue) "Undefined" "OverrideRootScale" null null))
      (bind _output_get (set `self.BP_Racket` _returnvalue_2))
      (set `/Game/Pong/GamePong/Blueprine/BP_Racket.Bp_Character` self _output_get)
      (`self.K2_AttachToComponent` _returnvalue_2 _right "None" "SnapToTarget" "SnapToTarget" "SnapToTarget" true)
      (`SceneComponent.SetVisibility` _right false false)
      (goto _label_2))
    (:`then_1`
      (bind _returnvalue_3 (`|SpawnActorFromClass` "/Game/Pong/GamePong/Blueprine/BP_Racket.BP_Racket_C" (`KismetMathLibrary.MakeTransform` _returnvalue) "Undefined" "OverrideRootScale" null null))
      (`self.K2_AttachToComponent` _returnvalue_3 _left "None" "SnapToTarget" "SnapToTarget" "SnapToTarget" true)
      (`self.K2_SetActorRotation` :`self` _returnvalue_3)
      (`SceneComponent.SetVisibility` _left false false))))

(fn `UserConstructionScript`)