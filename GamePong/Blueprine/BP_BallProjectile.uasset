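; Physics-driven Pong ball that clamps its top speed and publishes its position to a Material Parameter Collection every tick.
; The first hit while simulating marks it launched, after which low speed or too little movement along the X axis accumulates dead time.
; A dead ball blinks increasingly fast, then asks BPMain to spawn a new game and destroys itself with an explosion.
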(event `self.ReceiveTick`
  (params (DeltaSeconds :type "Float (single-precision)"))
  ;[1 1 1] Tick
  (set `self.Delta Seconds` DeltaSeconds)
  (`KismetMaterialLibrary.SetVectorParameterValue` "/Game/Assets/Materials/Collections/ParameterCollection.ParameterCollection" "Ball Position" (`KismetMathLibrary.Conv_VectorToLinearColor` (`self.K2_GetActorLocation`)))
  (bind _returnvalue (`PrimitiveComponent.GetPhysicsLinearVelocity` (`self.CollisionSphere`) "None"))
  (`PrimitiveComponent.SetAllPhysicsLinearVelocity` (`self.CollisionSphere`) (`KismetMathLibrary.ClampVectorSize` _returnvalue 0.0 800.0) false)
  (if (`self.Is Launched ?`)
    (if (or (< (`self.Get Speed`) (`self.Dead Ball Speed`)) (< (`KismetMathLibrary.Abs` (`KismetMathLibrary.Dot_VectorVector` (`self.Get Diretion`) (1.0 0.0 0.0))) (`self.Dead Dot Value`)))
      (set `self.Dead State Time` (+ (`self.Dead State Time`) (`self.Delta Seconds`)))
      (`|ExecutionSequence`
        (:`then_0`
          (if (> (`self.Dead State Time`) (/ (`self.Min Dead Time To Auto Destroy`) 2.0))
            (`KismetSystemLibrary.Delay` (`KismetMathLibrary.Lerp` 0.08 0.02 (`KismetMathLibrary.FClamp` (/ (`self.Dead State Time`) (`self.Min Dead Time To Auto Destroy`)))))
            (`SceneComponent.SetVisibility` (`self.Sphere_StaticMesh`) (not (`SceneComponent.bVisible` (`self.Sphere_StaticMesh`))) true)))
        (:`then_1`
          (`/Engine/EditorBlueprintResources/StandardMacros.CompareFloat` (`self.Dead State Time`) (`self.Min Dead Time To Auto Destroy`)
            (:`>`
              (`/Engine/EditorBlueprintResources/StandardMacros.DoOnce` false
                (:`Completed`
                  (`KismetSystemLibrary.Delay` 3.0)
                  (`/Game/Pong/GamePong/Blueprine/BP_MainGameActor.SpawnNewGameROS` (`self.BP_Main`))
                  (`self.K2_DestroyActor`)))))))
      (else
        (set `self.Dead State Time` 0.0)
        (`SceneComponent.SetVisibility` (`self.Sphere_StaticMesh`) true true)))))

(event `Enable Physics Simulation ROS`
  (bind _collisionsphere (`self.CollisionSphere`))
  ;[1 1 1] Set Physics and Velocity
  (`PrimitiveComponent.SetSimulatePhysics` _collisionsphere true)
  (`PrimitiveComponent.SetAllPhysicsLinearVelocity` _collisionsphere (0.0 0.0 0.0) false))

(event `self.ReceiveDestroyed`
  ;[1 1 1] Destroyball
  (`GameplayStatics.SpawnEmitterAtLocation` "/Game/StarterContent/Particles/P_Explosion.P_Explosion" (`self.K2_GetActorLocation`) (`KismetMathLibrary.RandomRotator` true) (0.5 0.5 0.5)))

(event `self.CollisionSphere.OnComponentHit`
  (params (HitComponent :type "PrimitiveComponent Object Reference") (OtherActor :type "Actor Object Reference") (OtherComp :type "PrimitiveComponent Object Reference") (NormalImpulse :type "Vector Structure") (Hit :type "HitResult Structure (by ref)"))
  ;[1 1 1] Hit
  (if (`SceneComponent.IsSimulatingPhysics` (`self.CollisionSphere`) "None")
    (set `self.Is Launched ?` true)))

(fn `UserConstructionScript`)